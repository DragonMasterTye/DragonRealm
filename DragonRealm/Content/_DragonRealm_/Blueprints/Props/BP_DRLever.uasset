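; BP_DRLever is a lever prop whose Interact event currently only adds KeycardTag to the instigator pawn's DRActionComponent active gameplay tags.
; A disconnected toggle graph would play or reverse a timeline that pitches the handle mesh.
; In that unused graph, finishing in the on state forwards the interaction to SelectedActor, or prints an error if none is valid.
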(event `DRGameplayInterface.Interact`
  (params (InstigatorPawn :type "Pawn Object Reference"))
  (`BlueprintGameplayTagLibrary.AddGameplayTag` (`DRActionComponent.ActiveGameplayTags` (`self.GetComponentByClass` InstigatorPawn "/Script/DragonRealm.DRActionComponent")) (`self.KeycardTag`)))

(fn `UserConstructionScript`)