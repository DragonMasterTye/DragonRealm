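; BP_DR_Lever is a toggleable lever prop that triggers another actor when switched on.
; Interact flips IsOn and plays or reverses the AnimateLever timeline, which drives the handle mesh's pitch.
; When the timeline finishes in the on state, it forwards Interact and the instigator pawn to SelectedActor through an interface message, or prints an error if none is valid.
; Switching off only animates the handle back, without notifying SelectedActor.
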(event `DR_GameplayInterface.Interact`
  (params (InstigatorPawn :type "Pawn Object Reference"))
  (bind _selectedactor (`self.SelectedActor`))
  (if (not (`self.bIsOn`))
    (set `self.bIsOn` true)
    (bind (_direction _pitch) (`Timeline|AnimateLever` :!via `PlayFromStart` :!label _label)
      (:`Update`
        (`SceneComponent.K2_SetRelativeRotation` (`self.HandleMesh`) (`KismetMathLibrary.MakeRotator` 0.0 _pitch) false false))
      (:`Finished`
        (if (`self.bIsOn`)
          (`/Engine/EditorBlueprintResources/StandardMacros.IsValid` _selectedactor
            (:`Is Valid`
              (message `DR_GameplayInterface.Interact` _selectedactor InstigatorPawn))
            (:`Is Not Valid`
              (`KismetSystemLibrary.PrintString` "Lever has no SelectedActor" true true (struct :`R` 1.0 :`A` 1.0) 10.0))))))
    (else
      (set `self.bIsOn` false)
      (goto _label :!via `ReverseFromEnd`))))

(fn `UserConstructionScript`)