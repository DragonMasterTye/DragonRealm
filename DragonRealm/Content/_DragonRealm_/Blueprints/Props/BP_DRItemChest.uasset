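; BP_DRItemChest is an item chest prop that shows its lid opening from the replicated LidOpened state.
; OnRepLidOpened calls the parent, then plays a timeline that pitches the lid mesh and activates a particle system when finished.
; If the chest is under a second old, the lid snaps open instead, skipping animation and particles.
; An unconnected keycard tag check with debug print remains in the graph but never runs.
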(event `self.OnRep_LidOpened`
  (`parent.OnRep_LidOpened`)
  (if (`self.bLidOpened`)
    (if (< (`self.GetGameTimeSinceCreation`) 1.0)
      (`SceneComponent.K2_SetRelativeRotation` (`self.LidMesh`) (`KismetMathLibrary.MakeRotator` 0.0 110.0) false false)
      (else
        (bind (_direction _pitch) (`Timeline|Timeline` :!via `PlayFromStart`)
          (:`Update`
            (`SceneComponent.K2_SetRelativeRotation` (`self.LidMesh`) (`KismetMathLibrary.MakeRotator` 0.0 _pitch) false false))
          (:`Finished`
            (`ActorComponent.Activate` (`self.ParticleSystem`) true)))))))

(fn `UserConstructionScript`)