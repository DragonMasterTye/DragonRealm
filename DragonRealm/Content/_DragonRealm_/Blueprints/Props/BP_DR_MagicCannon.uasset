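; BP_DR_MagicCannon is a turret prop that fires magic projectiles at the player.
; Every tick it rotates its Arrow component to face the first player pawn's location.
; A looping timer started on BeginPlay spawns a BP_DR_MagicProjectile_Basic at the Arrow's world transform every couple of seconds, with no range or line-of-sight check.
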(event `self.ReceiveBeginPlay`
  (`KismetSystemLibrary.K2_SetTimerDelegate` (delegate `OnTimerElapsed`) 2.0 true true))

(event `OnTimerElapsed`
  (`|SpawnActorFromClass` "/Game/_DragonRealm_/Blueprints/Abilities/Projectiles/BP_DR_MagicProjectile_Basic.BP_DR_MagicProjectile_Basic_C" (`SceneComponent.K2_GetComponentToWorld` (`self.Arrow`)) "AlwaysSpawn" "MultiplyWithRoot" self self))

(event `self.ReceiveTick`
  (params (DeltaSeconds :type "Float (single-precision)"))
  (bind _arrow (`self.Arrow`))
  (`SceneComponent.K2_SetWorldRotation` _arrow (`KismetMathLibrary.FindLookAtRotation` (`SceneComponent.K2_GetComponentLocation` _arrow) (`self.K2_GetActorLocation` (`GameplayStatics.GetPlayerPawn` 0))) false false))

(fn `UserConstructionScript`)