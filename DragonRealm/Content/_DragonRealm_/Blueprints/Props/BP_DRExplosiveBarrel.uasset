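; BP_DRExplosiveBarrel is an explosive barrel prop that detonates when an actor overlaps it.
; The overlap is handled only on authority, which multicasts the explosion and gives the barrel a short life span before destruction.
; The explosion fires the force component's impulse, hides the mesh, disables its collision, and spawns a scaled-up particle effect and sound at the barrel's location.
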(event `self.OnActorOverlap`
  (params (OverlappedComponent :type "PrimitiveComponent Object Reference") (OtherActor :type "Actor Object Reference") (OtherComponent :type "PrimitiveComponent Object Reference") (OtherBodyIndex :type Integer) (bFromSweep :type Boolean) (SweepResult :type "HitResult Structure (by ref)"))
  (`/Engine/EditorBlueprintResources/ActorMacros.Switch Has Authority`
    (:`Authority`
      (`self.MULTICAST_Explode`)
      (`self.SetLifeSpan` 2.0))))

(event `MULTICAST_Explode`
  (`self.Explode`))

(event `self.Explode`
  (bind _meshcomponent (`self.MeshComponent`))
  (`RadialForceComponent.FireImpulse` (`self.ForceComponent`))
  (`SceneComponent.SetVisibility` _meshcomponent false false)
  (`PrimitiveComponent.SetCollisionEnabled` _meshcomponent "NoCollision")
  (`GameplayStatics.SpawnEmitterAtLocation` "/Game/ExampleContent/Effects/P_Explosion.P_Explosion" (`self.K2_GetActorLocation`) (struct) (10.0 10.0 10.0))
  (`GameplayStatics.PlaySoundAtLocation` "/Game/Marketplace/LowPolyAnimatedModernGuns/Audio/Cues/Explosions/SC_LPAMG_Explosion_Grenade_04.SC_LPAMG_Explosion_Grenade_04" (`self.K2_GetActorLocation`) (struct) 1.0 1.0 0.0 null null null null))

(fn `UserConstructionScript`)