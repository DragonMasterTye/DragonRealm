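; BP_DRBonfire is a bonfire prop that lights when interacted with and acts as a save point.
; Interact sets FireActive, writes the save game through DRGameModeBase, prints a confirmation and updates the flames.
; OnActorLoaded calls the same UpdateFlames event, which activates the particle system whenever FireActive is true.
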(event `DRGameplayInterface.Interact`
  (params (InstigatorPawn :type "Pawn Object Reference"))
  (set `self.bFireActive` true)
  (bind _asdrgame_mode_base (cast `DRGameModeBase` (`GameplayStatics.GetGameMode`)))
  (`DRGameModeBase.WriteSaveGame` _asdrgame_mode_base "DRSaveGame")
  (`KismetSystemLibrary.PrintString` "GAME SAVED")
  (`self.UpdateFlames`))

(event `DRGameplayInterface.OnActorLoaded`
  (`self.UpdateFlames`))

(event `UpdateFlames`
  (if (`self.bFireActive`)
    (`ActorComponent.Activate` (`self.ParticleSystem`) false)))

(fn `UserConstructionScript`)