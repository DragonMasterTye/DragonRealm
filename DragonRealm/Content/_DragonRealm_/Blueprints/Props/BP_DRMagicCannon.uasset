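; BP_DRMagicCannon is a magic cannon prop that automatically fires basic magic projectiles at the player.
; An Arrow component serves as the muzzle, rotated every Tick to face player pawn 0.
; If TurnOn is set at BeginPlay, a looping one-second timer spawns projectiles from the Arrow transform, with the cannon as owner and instigator.
; Aiming runs regardless of TurnOn, with no range or line-of-sight check.
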(event `self.ReceiveBeginPlay`
  (if (`self.bTurnOn`)
    (`KismetSystemLibrary.K2_SetTimerDelegate` (delegate `OnTimerElapsed`) 1.0 true true)))

(event `OnTimerElapsed`
  (`|SpawnActorFromClass` "/Game/_DragonRealm_/Blueprints/Actions/Projectiles/BP_DRMagicProjectile_Basic.BP_DRMagicProjectile_Basic_C" (`SceneComponent.K2_GetComponentToWorld` (`self.Arrow`)) "AlwaysSpawn" "MultiplyWithRoot" self self))

(event `self.ReceiveTick`
  (params (DeltaSeconds :type "Float (single-precision)"))
  (bind _arrow (`self.Arrow`))
  (`SceneComponent.K2_SetWorldRotation` _arrow (`KismetMathLibrary.FindLookAtRotation` (`SceneComponent.K2_GetComponentLocation` _arrow) (`self.K2_GetActorLocation` (`GameplayStatics.GetPlayerPawn` 0))) false false))

(fn `UserConstructionScript`)