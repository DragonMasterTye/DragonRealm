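; Maze generator Blueprint named for the binary tree algorithm, which so far only lays out the floor grid.
; GenerateMaze clears the center instanced static mesh, then adds tiles spaced by TileSize in a square grid, using NumberOfTilesX for both axes.
; Disconnected nodes for filling a coordinate list and adding wall instances never run, so no maze carving or wall placement happens.
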(event `GenerateMaze`
  (bind _instancedstaticcenter (`self.InstancedStaticCenter`))
  (`InstancedStaticMeshComponent.ClearInstances` _instancedstaticcenter)
  (for _index (range (+ (`self.NumberOfTilesX`) 1))
    (for _index_2 (range (+ (`self.NumberOfTilesX`) 1))
      (`InstancedStaticMeshComponent.AddInstance` _instancedstaticcenter (`KismetMathLibrary.MakeTransform` (`KismetMathLibrary.MakeVector` (* _index_2 (`self.TileSize`)) (* _index (`self.TileSize`))) (struct) (1.0 1.0 1.0)) false))))

(fn `UserConstructionScript`)