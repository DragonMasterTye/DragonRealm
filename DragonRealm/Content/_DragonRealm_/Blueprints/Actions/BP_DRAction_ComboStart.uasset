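; BP_DRAction_ComboStart is an action that serves as the entry point for a two-step combo, driven by gameplay tags on the owning action component.
; Without a Status.Combo tag, it starts itself and triggers Combo01; with Status.Combo.01 active, it triggers Combo02 instead.
; A handler stops the action once Status.Combo.01 is absent when an action stops, but its delegate binding is disconnected.
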(event `self.StartAction`
  (params (Instigator :type "Actor Object Reference"))
  (bind _output_get (set `self.Instigator` Instigator))
  (if (`BlueprintGameplayTagLibrary.HasTag` (`DRActionComponent.ActiveGameplayTags` (`self.GetOwningComponent`)) (struct :`TagName` "Status.Combo") true)
    (if (`BlueprintGameplayTagLibrary.HasTag` (`DRActionComponent.ActiveGameplayTags` (`self.GetOwningComponent`)) (struct :`TagName` "Status.Combo.01") true)
      (`DRActionComponent.StartActionByName` (`self.GetOwningComponent`) (`self.Instigator`) "Combo02"))
    (else
      (`parent.StartAction` _output_get)
      (`DRActionComponent.StartActionByName` (`self.GetOwningComponent`) _output_get "Combo01"))))

(event `OnActionStopped_Event`
  (params (OwningComponent :type "DRActionComponent Object Reference") (Action :type "DRAction Object Reference"))
  (if (not (`BlueprintGameplayTagLibrary.HasAnyTags` (`DRActionComponent.ActiveGameplayTags` (`self.GetOwningComponent`)) (`BlueprintGameplayTagLibrary.MakeLiteralGameplayTagContainer` (struct :`GameplayTags` (struct :`(TagName` "Status.Combo.01") :`(TagName` "Status.Combo.02"))))))
    (`self.StopAction` (`self.Instigator`))))