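; Basic magic projectile for DragonRealm that damages actors it overlaps and inflicts a damage-over-time effect.
; On overlap, the server skips the instigator and applies directional damage using the sweep hit result.
; It then adds the DoT effect to targets that have a DRActionComponent.
; The parent overlap handler runs afterward on every machine, including when the instigator is hit.
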(event `self.OnActorOverlap`
  (params (OverlappedComponent :type "PrimitiveComponent Object Reference") (OtherActor :type "Actor Object Reference") (OtherComponent :type "PrimitiveComponent Object Reference") (OtherBodyIndex :type Integer) (bFromSweep :type Boolean) (SweepResult :type "HitResult Structure (by ref)"))
  (bind _returnvalue (`self.GetComponentByClass` OtherActor "/Script/DragonRealm.DRActionComponent"))
  (`|ExecutionSequence`
    (:`then_0`
      (`/Engine/EditorBlueprintResources/ActorMacros.Switch Has Authority`
        (:`Authority`
          (if (!= (`self.GetInstigator`) OtherActor)
            (`DRGameplayFunctionLibrary.DR_ApplyDirectionalDamage` (`self.GetInstigator`) OtherActor (`self.Damage`) SweepResult)
            (`/Engine/EditorBlueprintResources/StandardMacros.IsValid` _returnvalue
              (:`Is Valid`
                (`DRActionComponent.AddAction` _returnvalue (`self.GetInstigator`) "/Game/_DragonRealm_/Blueprints/Actions/BP_DREffect_DoT.BP_DREffect_DoT_C")))))))
    (:`then_1`
      (`parent.OnActorOverlap` OverlappedComponent OtherActor OtherComponent OtherBodyIndex bFromSweep SweepResult))))

(fn `UserConstructionScript`)