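; Test player controller for DragonRealm that sets up the main HUD and offers a debug save shortcut.
; On BeginPlay, the local controller creates WBP_DRMainHUD, adds it to the viewport and switches input to game only.
; Pressing L casts the game mode to DRGameModeBase and writes the DRSaveGame save slot.
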(event `self.ReceiveBeginPlay`
  (if (`self.IsLocalController`)
    (bind _returnvalue (`|CreateWidget` "/Game/_DragonRealm_/Blueprints/UI/WBP_DRMainHUD.WBP_DRMainHUD_C" self))
    (`UserWidget.AddToViewport` _returnvalue 0)
    (`WidgetBlueprintLibrary.SetInputMode_GameOnly` self)))

(event `Key|L`
  (params (Key :type "Key Structure"))
  (:`Pressed`
    (bind _asdrgame_mode_base (cast `DRGameModeBase` (`GameplayStatics.GetGameMode`)))
    (`DRGameModeBase.WriteSaveGame` _asdrgame_mode_base "DRSaveGame")))

(fn `UserConstructionScript`)